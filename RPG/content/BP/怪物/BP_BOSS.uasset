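; BP_BOSS is a boss monster that chases BP_Blue on sight, attacks in melee, takes damage and dies.
; PawnSensing drives AIMoveTo, then a DoOnce-gated attack montage that re-arms two seconds after completing.
; HP is seeded from a BW_BOSS widget; 受傷BOSS subtracts damage and plays hit or dying montages.
; Tick polls HP to flag death and destroy the actor after a delay; random wandering logic is disconnected.
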(event `self.PawnSensing.OnSeePawn`
  (params (Pawn :type "Pawn Object Reference"))
  ;[1 1 1] 怪物追蹤+自動攻擊
  (if (not (`self.是否有攻擊`))
    (bind _asbp_blue (cast `/Game/BP/角色/BP_Blue` Pawn))
    (`|AIMoveTo` self (0.0 0.0 0.0) _asbp_blue
      (:`OnSuccess`
        (`/Engine/EditorBlueprintResources/StandardMacros.DoOnce` false :!label _label
          (:`Completed`
            (`|PlayMontage` (`self.Mesh`) "/Game/Animations/怪物/Aattack_BOSS2_Montage.Aattack_BOSS2_Montage"
              (:`then`
                (set `self.是否有攻擊` true))
              (:`OnCompleted`
                (set `self.是否有攻擊` false)
                (`KismetSystemLibrary.Delay` 2.0)
                (goto _label :!via `Reset`)))))))))

(event `self.ReceiveBeginPlay`
  (bind _returnvalue (`|CreateWidget` "/Game/BP/怪物/BW_BOSS.BW_BOSS_C"))
  (bind _output_get (set `/Game/BP/怪物/BW_BOSS.BOSS 血量` (`/Game/BP/怪物/BW_BOSS.BOSS_HP` _returnvalue) _returnvalue))
  (set `self.HP_BOSS_TEST` _output_get))

(event `self.ReceiveTick`
  (params (DeltaSeconds :type "Float (single-precision)"))
  (if (<= (`self.HP_BOSS_TEST`) 0.0)
    (set `self.是否有死亡` true)
    (`/Engine/EditorBlueprintResources/StandardMacros.DoOnce` false
      (:`Completed`
        (`KismetSystemLibrary.Delay` 4.0)
        (`self.K2_DestroyActor` self)))))

(fn `UserConstructionScript`)

(fn `受傷_BOSS`
  (params (`傷害值` :type "Float (double-precision)"))
  (bind _hp_boss_test (`self.HP_BOSS_TEST`))
  (if (not (`self.是否有死亡`))
    (set `self.HP_BOSS_TEST` (- (`self.HP_BOSS_TEST`) `傷害值`))
    (`self.PlayAnimMontage` self "/Game/Animations/怪物/BOSS_hit_Montage.BOSS_hit_Montage" 1.0 "None")
    (`KismetSystemLibrary.PrintString` (`KismetStringLibrary.Conv_DoubleToString` _hp_boss_test))
    (if (<= _hp_boss_test 0.0)
      (`self.PlayAnimMontage` self "/Game/Animations/怪物/BOSS_Dying_Montage.BOSS_Dying_Montage" 1.0 "None"))))